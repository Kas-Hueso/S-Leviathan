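; BPC_Life is a component that holds a life (health) value for the actor that owns it.
; On BeginPlay it sets the current Life to TotalLife.
; It exposes functions to read, add to and subtract from Life, with no clamping, death check or change event.
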(event EventBeginPlay
  (Variables|Default|SetLife (Variables|Default|GetTotal%20Life)))

(fn GetLife
  (return (Variables|Default|GetLife)))

(fn AddLife
  (params (Add%20Value :type Float%20%28double-precision%29))
  (Variables|Default|SetLife (+ Add%20Value (Variables|Default|GetLife))))

(fn SubtractLife
  (params (Subtract%20Life :type Float%20%28double-precision%29))
  (Variables|Default|SetLife (- (Variables|Default|GetLife) Subtract%20Life)))