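; BP_Vigia is a flying enemy with sight perception and a spotlight, which runs the AI_EnemyBehaviors behavior tree on BeginPlay.
; Custom timer-driven events pick random traced points to fly toward until a player-tagged Target is set.
; FlytoPlayer turns the light yellow and sphere-traces for the player, but its steering is disconnected.
; Nothing connected in this graph starts detection or the roaming loop, and several older movement attempts remain unwired.
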(event OnPerceptionUpdated(AIPerception)
  (params (UpdatedActors :type Array%20of%20Actor%20Object%20References)))

(event Custom|Detect%20Player
  (for _array_element (Class|AIPerceptionComponent|GetKnownPerceivedActors (Variables|Default|GetAIPerception) "/Script/AIModule.AISense_Sight")
    (if (Actor|ActorHasTag _array_element "Player")
      (Variables|Default|SetTarget _array_element)
      (else
        (Variables|Default|SetTarget 0)))))

(event Custom|Move%20To
  (Variables|Default|GetTarget
    (:then
      (bind _returnvalue (Utilities|Time|SetTimerbyEvent (delegate Custom|Fly%20to%20Player) 0.01 true)))
    (:else
      (bind (_outhit _returnvalue_2) (Collision|LineTraceForObjects (Transformation|GetActorLocation) (* (+ (* (Transformation|GetActorForwardVector) (Math|Random|RandomIntegerinRange -1 1)) (* (Transformation|GetActorRightVector) (Math|Random|RandomIntegerinRange -1 1)) (* (Transformation|GetActorUpVector) (Math|Random|RandomIntegerinRange -1 1))) (Math|Random|RandomFloatinRange 2e+03 6e+03)) (Utilities|Array|MakeArray "ObjectTypeQuery1" "ObjectTypeQuery2") false 0 "None" :!label _label))
      (if (> (Math|Vector|Distance(Vector) (Variables|Default|GetLocation) (.ImpactPoint (Collision|BreakHitResult _outhit))) 1e+03)
        (Variables|Default|SetLocation (select _returnvalue_2 (.ImpactPoint (Collision|BreakHitResult _outhit)) (.TraceEnd (Collision|BreakHitResult _outhit))))
        (bind _returnvalue_3 (Utilities|Time|SetTimerbyEvent (delegate Custom|Fly%20to%20random%20location) 0.01 true))
        (else
          (goto _label))))))

(event Custom|Fly%20to%20random%20location
  (bind _returnvalue (Transformation|GetActorLocation))
  (bind _location (Variables|Default|GetLocation))
  (bind _location_2 (Variables|Default|GetLocation))
  (bind _returnvalue_2 (Math|Rotator|FindLookatRotation _returnvalue _location_2))
  (Variables|Default|GetTarget
    (:then
      (Utilities|Time|ClearandInvalidateTimerbyHandle (stale Custom|Move%20To _returnvalue_3))
      (Utilities|Time|SetTimerbyEvent (delegate Custom|Move%20To) 0.1 :!label _label)
      (Pawn|Components|CharacterMovement|SetMovementMode (Variables|Character|GetCharacterMovement) "MOVE_Flying" 0))
    (:else
      (bind (_outhit _returnvalue_3) (Collision|SphereTraceForObjects _location _location 1e+02 (Utilities|Array|MakeArray "ObjectTypeQuery3") false 0 "Persistent" false))
      (Pawn|Input|AddMovementInput (Math|Vector|GetForwardVector (Math|Rotator|MakeRotator 0.0 (.pitch _returnvalue_2) (.yaw _returnvalue_2))) 1.0 false)
      (if _returnvalue_3
        (if (Actor|ActorHasTag (.HitActor (Collision|BreakHitResult _outhit)) "Enemy")
          (Utilities|Time|ClearandInvalidateTimerbyHandle (stale Custom|Move%20To _returnvalue_3))
          (Utilities|FlowControl|RetriggerableDelay 3.0)
          (goto _label))))))

(event Custom|Fly%20to%20Player
  (Rendering|Components|Light|SetLightColor (Variables|Default|GetSpotLight) "(R=1.000000,G=0.920964,B=0.000000,A=1.000000)" true)
  (bind (_outhit _returnvalue) (Collision|SphereTraceForObjects (Transformation|GetActorLocation) (* (Transformation|GetActorForwardVector) 1e+02) 1e+02 (Utilities|Array|MakeArray "ObjectTypeQuery3") false 0 "None"))
  (if _returnvalue
    (if (Actor|ActorHasTag (.HitActor (Collision|BreakHitResult _outhit)) "Player")
      (Utilities|Time|ClearandInvalidateTimerbyHandle (stale Custom|Move%20To _returnvalue))
      (Utilities|FlowControl|RetriggerableDelay 1.0)
      (Utilities|Time|SetTimerbyEvent (delegate Custom|Move%20To) 0.1)
      (Pawn|Components|CharacterMovement|SetMovementMode (Variables|Character|GetCharacterMovement) "MOVE_Flying" 0))))

(event EventBeginPlay
  (Pawn|Components|CharacterMovement|SetMovementMode (Variables|Character|GetCharacterMovement) "MOVE_Flying" 0)
  (AI|RunBehaviorTree (AI|GetAIController self) "/Game/COM/AI_EnemyBehaviors.AI_EnemyBehaviors"))

(fn ConstructionScript)