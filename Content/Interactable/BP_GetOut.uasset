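; BP_GetOut is an exit trigger that ends the game with a good or bad ending level.
; When the first-person character overlaps its Box, it reads the money total from that character's BPCObtainLoot component.
; Exactly 500 opens Lvl_GoodEnding, then shows the cursor, sets UI-only input and pauses the game.
; Any other amount, higher or lower, only opens Lvl_BadEnding.
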(event OnComponentBeginOverlap(Box)
  (params (OverlappedComponent :type Primitive%20Component%20Object%20Reference) (OtherActor :type Actor%20Object%20Reference) (OtherComp :type Primitive%20Component%20Object%20Reference) (OtherBodyIndex :type Integer) (bFromSweep :type Boolean) (SweepResult :type Hit%20Result%20Structure%20%28by%20ref%29))
  (bind _returnvalue (Game|GetPlayerController 0))
  (bind _asbp_first_person_character (Utilities|Casting|CastToBP_FirstPersonCharacter OtherActor))
  (bind _money (Default|GetAmountOfMoney (Variables|/Game/FirstPerson/Blueprints/BP_FirstPersonCharacter.BP_FirstPersonCharacter_C|GetBPC_ObtainLoot _asbp_first_person_character)))
  (if (== _money 500)
    (Game|OpenLevel(byName) "Lvl_GoodEnding")
    (Variables|/Script/Engine.PlayerController|SetbShowMouseCursor _returnvalue true)
    (Input|SetInputModeUIOnly _returnvalue 0 "DoNotLock" false)
    (Game|SetGamePaused true)
    (else
      (Game|OpenLevel(byName) "Lvl_BadEnding"))))

(event EventBeginPlay)

(event Collision|EventActorBeginOverlap
  (params (OtherActor :type Actor%20Object%20Reference)))

(event EventTick
  (params (DeltaSeconds :type Float%20%28single-precision%29)))

(fn ConstructionScript)