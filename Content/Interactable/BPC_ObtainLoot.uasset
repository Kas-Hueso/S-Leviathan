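; BPC_ObtainLoot is a loot component that keeps running totals of collected money and weight.
; Light, normal and heavy add functions each raise money by a fixed, increasing amount and send the new total to the game mode as a score message.
; Only the light function also increases weight and sends a weight message.
; Getters expose both totals, and the event graph has no active logic.
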(event EventBeginPlay)

(event EventTick
  (params (DeltaSeconds :type Float%20%28single-precision%29)))

(fn AddMoneyLight
  (Utilities|FlowControl|Sequence
    (:then_0
      (bind _output_get (Variables|Default|SetAmount%20of%20Money (+ (Variables|Default|GetAmount%20of%20Money) 50)))
      (Class|BPIManagerFunctions|AddScore(Message) (Game|GetGameMode) _output_get))
    (:then_1
      (bind _output_get_2 (Variables|Default|SetAmount%20of%20Weight (+ (Variables|Default|GetAmount%20of%20Weight) 100)))
      (Class|BPIManagerFunctions|AddWeight(Message) (Game|GetGameMode) _output_get_2))))

(fn AddMoneyNormal
  (bind _output_get (Variables|Default|SetAmount%20of%20Money (+ (Variables|Default|GetAmount%20of%20Money) 150)))
  (Class|BPIManagerFunctions|AddScore(Message) (Game|GetGameMode) _output_get))

(fn AddMoneyHeavy
  (bind _output_get (Variables|Default|SetAmount%20of%20Money (+ (Variables|Default|GetAmount%20of%20Money) 250)))
  (Class|BPIManagerFunctions|AddScore(Message) (Game|GetGameMode) _output_get))

(fn GetAmountOfMoney
  (return (Variables|Default|GetAmount%20of%20Money)))

(fn GetAmountOfWeight
  (return (Variables|Default|GetAmount%20of%20Weight)))