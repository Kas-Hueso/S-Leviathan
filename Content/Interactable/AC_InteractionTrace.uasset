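; Actor component that lets the player focus and interact with BP_InteractionArea actors in view.
; Each tick it line-traces forward from the player camera on Visibility, toggling focus on and off as the hit actor changes.
; TryToInteract sends OnInteractMessage to the focused area's parent actor through InteractOnServer.
; Only areas without a positive InteractDuration trigger this; timed interaction has no handling here.
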(event Custom|TryToInteract
  (params (In :type Boolean))
  (if In
    (if (Variables|Default|GetIsTracingInteractionArea)
      (bind _output_get (Variables|Default|SetInteract%20Duration (Variables|/Game/Interactable/BP_InteractionArea.BP_InteractionArea_C|GetInteractDuration (Variables|Default|GetFocusedInteractionArea))))
      (if (not (> _output_get 0.0))
        (CallFunction|InteractonServer (Variables|Default|GetFocusedInteractionArea))))))

(event Custom|InteractOnServer
  (params (InteractionArea :type BP%20Interaction%20Area%20Object%20Reference))
  (Class|BPIInteraction|OnInteract(Message) (Actor|GetParentActor InteractionArea)))

(event EventTick
  (params (DeltaSeconds :type Float%20%28single-precision%29))
  (CallFunction|Trace))

(fn Trace
  (bind _returnvalue (Game|GetPlayerCameraManager 0))
  (bind _returnvalue_2 (Transformation|GetActorLocation _returnvalue))
  (bind (_outhit _returnvalue_3) (Collision|LineTraceByChannel _returnvalue_2 (+ _returnvalue_2 (* (Math|Vector|GetForwardVector (Transformation|GetActorRotation _returnvalue)) (Variables|Default|GetLength))) "TraceTypeQuery1" false 0 "None"))
  (if _returnvalue_3
    (if (!= (Variables|Default|GetFocused%20Actor) (.HitActor (Collision|BreakHitResult _outhit)))
      (Variables|Default|SetFocused%20Actor (.HitActor (Collision|BreakHitResult _outhit)))
      (CallFunction|TraceInteractionArea (== (Utilities|GetClass (.HitActor (Collision|BreakHitResult _outhit))) "/Game/Interactable/BP_InteractionArea.BP_InteractionArea_C")))
    (else
      (CallFunction|TraceInteractionArea false))))

(fn TraceInteractionArea
  (params (Trace :type Boolean))
  (if Trace
    (if (Variables|Default|GetIsTracingInteractionArea)
      (bind _focusedinteractionarea (Variables|Default|GetFocusedInteractionArea)
        (:then
          (Default|ToggleFocus _focusedinteractionarea false))
        (:else))
      (else
        (bind _focused_actor (Variables|Default|GetFocused%20Actor)
          (:then
            _)
          (:else))))
    (bind _asbp_interaction_area (Utilities|Casting|CastToBP_InteractionArea _focused_actor))
    (bind _output_get (Variables|Default|SetFocusedInteractionArea _asbp_interaction_area))
    (Default|ToggleFocus _output_get true)
    (Variables|Default|SetIsTracingInteractionArea true)
    (elif (Variables|Default|GetIsTracingInteractionArea)
      (Variables|Default|SetIsTracingInteractionArea false)
      (bind _focusedinteractionarea_2 (Variables|Default|GetFocusedInteractionArea)
        (:then
          (Default|ToggleFocus _focusedinteractionarea_2 false)
          (Variables|Default|SetFocused%20Actor 0)
          (Variables|Default|SetFocusedInteractionArea 0))
        (:else)))))