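; BP_HeavyLoot is an interactable loot item with a prize value and weight that is collected on interaction.
; Focus toggles custom depth on its cube, and the actor supplies its interaction widget.
; OnInteract calls InteractOnServer to flip InteractToggle, whose RepNotify sends score, weight and treasure radar messages to the GameMode, then destroys the actor when true.
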(event Custom|Interact%20On%20Server
  (Variables|Default|SetInteractToggle (not (Variables|Default|GetInteractToggle))))

(event EventBeginPlay)

(event Collision|EventActorBeginOverlap
  (params (OtherActor :type Actor%20Object%20Reference)))

(event EventTick
  (params (DeltaSeconds :type Float%20%28single-precision%29)))

(event EventInterfaceToggleFocus
  (params (Focus :type Boolean))
  (Rendering|SetRenderCustomDepth (Variables|Default|GetCube) Focus))

(event EventOnInteract
  (CallFunction|InteractonServer))

(fn ConstructionScript)

(fn OnRepInteractToggle
  (bind _returnvalue (Game|GetGameMode))
  (if (Variables|Default|GetInteractToggle)
    (Class|BPIManagerFunctions|AddScore(Message) _returnvalue (Variables|Default|GetPrize))
    (Class|BPIManagerFunctions|AddWeight(Message) _returnvalue (Variables|Default|GetWeight))
    (Class|BPIManagerFunctions|UpdateTreasureRadar(Message) _returnvalue)
    (Actor|DestroyActor)))

(fn GetInteractionWidget
  (return (Variables|Default|GetWidget)))